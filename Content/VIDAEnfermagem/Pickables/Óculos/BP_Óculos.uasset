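; BP_Óculos is a pickable pair of glasses that the player puts on by bringing it to the head of BP_FloatingHands.
; Setup runs the parent BeginPlay and sets grip transforms for each hand.
; On head overlap it hides the mesh, detaches from the hand, attaches to the head and notifies the FSM via GlassesPutOn.
; The removal logic with its timed re-enable is unconnected and never runs.
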(event OnComponentBeginOverlap(Oculos-def)
  (params (OverlappedComponent :type Primitive%20Component%20Object%20Reference) (OtherActor :type Actor%20Object%20Reference) (OtherComp :type Primitive%20Component%20Object%20Reference) (OtherBodyIndex :type Integer) (bFromSweep :type Boolean) (SweepResult :type Hit%20Result%20Structure%20%28by%20ref%29))
  (bind _rootcomponent (Variables|Transformation|GetRootComponent))
  (if (not (Variables|Default|Getoculos%20colocado))
    (bind _asbp_floating_hands (Utilities|Casting|CastToBP_FloatingHands OtherActor))
    (if (== (Variables|/Game/VIDAEnfermagem/Characters/Player/BP_FloatingHands.BP_FloatingHands_C|GetCabeça _asbp_floating_hands) OtherComp)
      (Variables|Default|Setoculos%20colocado true)
      (Development|PrintString "Óculos colocado")
      (Rendering|SetVisibility (Variables|Default|GetOculos-def) false false)
      (CallFunction|DetachfromHand)
      (Transformation|AttachComponentToComponent _rootcomponent OtherComp "None" "KeepRelative" "KeepRelative" "KeepRelative" true)
      (Transformation|SetRelativeLocationAndRotation _rootcomponent "30.000000,0.000000, 0" "0, 0, 0" false false)
      (Default|GlassesPuton (Variables|Default|GetFSM)))))

(event EventBeginPlay
  (CallFunction|Setup))

(event Collision|EventActorBeginOverlap
  (params (OtherActor :type Actor%20Object%20Reference)))

(event EventTick
  (params (DeltaSeconds :type Float%20%28single-precision%29)))

(fn ConstructionScript)

(fn Setup
  (bind _transformpadrao (Variables|Default|GettransformPadrao))
  (|CallParentFunction)
  (Variables|Default|SettransformMaoDireita (Math|Transform|MakeTransform "-9.200000,11.710000,10.340000" "-60.779999,114.360001,81.570000" (.scale _transformpadrao)))
  (Variables|Default|SettransformMaoEsquerda (Math|Transform|MakeTransform "12.000000,-4.000000,-5.000000" "-80.000000, 0, 0" (.scale _transformpadrao))))

(fn AtivaColocação
  (Variables|Default|Setoculos%20colocado false))