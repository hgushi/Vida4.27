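; Actor that renders Leap Motion tracked low-poly hands, driving separate Left and Right skeletal meshes from tracking data.
; On BeginPlay it scales its origin by world-to-meters so hands keep a constant size.
; Each tracking frame passes per-hand data to the matching anim blueprint, falling back to a second anim class such as the stretch variant.
; Tracking visibility changes toggle each mesh's visibility and overlap events.
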(event OnLeftHandVisibilityChanged(Leap)
  (params (bIsVisible :type Boolean))
  (bind _left (Variables|Default|GetLeft))
  ;[1 1 1] Sync mesh visibility with tracking visibility updates
  (Development|SetHiddeninGame _left (not bIsVisible) false)
  (Variables|/Script/Engine.PrimitiveComponent|SetbGenerateOverlapEvents _left bIsVisible))

(event OnRightHandVisibilityChanged(Leap)
  (params (bIsVisible :type Boolean))
  (bind _right (Variables|Default|GetRight))
  ;[1 1 1] Sync mesh visibility with tracking visibility updates
  (Development|SetHiddeninGame _right (not bIsVisible) false)
  (Variables|/Script/Engine.PrimitiveComponent|SetbGenerateOverlapEvents _right bIsVisible))

(event OnLeapTrackingData(Leap)
  (params (Frame :type %20Structure%20%28by%20ref%29))
  (for _array_element (Utilities|Struct|Break Frame)
    ;[1 1 1] Set Animation Data for each hand
    (switch Utilities|FlowControl|Switch|Switchon (Utilities|Struct|Break _array_element)
      (:LEAP_HAND_LEFT
        (CallFunction|SetLeftAnim _array_element))
      (:LEAP_HAND_RIGHT
        (CallFunction|SetRightAnim _array_element)))))

(event EventBeginPlay
  (Transformation|SetRelativeScale3D (Variables|Default|GetOrigin) (Math|Conversions|ToVector(Float) (/ (Class|HeadMountedDisplayFunctionLibrary|GetWorldtoMetersScale) 1e+02))) ; Hands are always same size
)

(fn ConstructionScript)

(fn SetLeftAnim
  (params (HandData :type %20Structure))
  (bind _left (Variables|Default|GetLeft))
  (bind _returnvalue (Components|SkeletalMesh|GetAnimInstance _left))
  (bind _asleap_low_poly_left_stretch_anim_bp (Utilities|Casting|CastTo _returnvalue)
    (:then
      (CallFunction|SetAnimData _asleap_low_poly_left_stretch_anim_bp HandData))
    (:CastFailed
      (bind _ascustom_leap_low_poly_left_stretch_anim_bp (Utilities|Casting|CastTo _returnvalue))
      (CallFunction|SetAnimData _ascustom_leap_low_poly_left_stretch_anim_bp HandData))))

(fn SetRightAnim
  (params (HandData :type %20Structure))
  (bind _right (Variables|Default|GetRight))
  (bind _returnvalue (Components|SkeletalMesh|GetAnimInstance _right))
  (bind _asleap_low_poly_right_stretch_anim_bp (Utilities|Casting|CastTo _returnvalue)
    (:then
      (CallFunction|SetAnimData _asleap_low_poly_right_stretch_anim_bp HandData))
    (:CastFailed
      (bind _ascustom_leap_low_poly_right_stretch_anim_bp (Utilities|Casting|CastToCustomLeapLowPolyRightStretchAnimBP _returnvalue))
      (Default|SetAnimData _ascustom_leap_low_poly_right_stretch_anim_bp HandData))))