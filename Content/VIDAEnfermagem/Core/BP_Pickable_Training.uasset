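; Base pickable training object that exposes grab-related state to the floating-hands player pawn, BP_FloatingHands_Training.
; On BeginPlay it stores its root's relative transform and caches a reference to that pawn.
; Getters return the default and per-hand transforms, the grab-enabled flag and the tray trigger used for immediate release.
; A left-or-right macro compares display names with the pawn's held objects to report right-hand attachment.
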(event EventBeginPlay
  (Variables|Default|SettransformPadrao (Transformation|GetRelativeTransform (Variables|Default|GetDefaultSceneRoot)))
  (CallFunction|SetarReferências))

(event Collision|EventActorBeginOverlap
  (params (OtherActor :type Actor%20Object%20Reference)))

(event EventTick
  (params (DeltaSeconds :type Float%20%28single-precision%29)))

(fn ConstructionScript)

(fn GetTransformPadrao
  (return (Variables|Default|GettransformPadrao)))

(fn GetTransformMaoDireita
  (return (Variables|Default|GettransformMaoDireita)))

(fn GetTransformMaoEsquerda
  (return (Variables|Default|GettransformMaoEsquerda)))

(fn GetPegarAtivado
  (return (Variables|Default|GetpegarAtivado)))

(fn GetSoltarImediatamente
  (return (Variables|Default|GettriggerBandeja)))

(fn SetarReferências
  (while (not (Variables|Default|GetreferênciasSetadas))
    (if (Utilities|IsValid (Variables|Default|GetjogadorReferência))
      _
      (else
        (bind _outactors (Actor|GetAllActorsOfClass "/Game/VIDAEnfermagem/Characters/Player/BP_FloatingHands_Training.BP_FloatingHands_Training_C"))
        (Variables|Default|SetjogadorReferência (Utilities|Array|Get(acopy) _outactors))))
    (Variables|Default|SetreferênciasSetadas (Utilities|IsValid (Variables|Default|GetjogadorReferência)))))

(fn IsAttachedtoRight
  (Utilities|EsquerdaOuDireita
    (:Direita
      (return true))
    (:Esquerda
      (return false))))